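; A document virus projectile actor for SpaceEater that disrupts the player's open documents on contact.
; On BeginPlay it randomly picks one of two shot materials for its mesh.
; When its box overlaps a SpaceEater pawn, it calls the game state to refresh docs, then close documents and user files.
; The graph contains no movement or self-destruction logic.
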(event `self.ReceiveBeginPlay`
  (bind _staticmeshcomponent (`self.StaticMeshComponent`))
  (if (`KismetMathLibrary.RandomBool`)
    (`PrimitiveComponent.SetMaterial` _staticmeshcomponent 0 "/Game/Materials/Shoot1_Mat.Shoot1_Mat")
    (else
      (`PrimitiveComponent.SetMaterial` _staticmeshcomponent 0 "/Game/Materials/Shoot0_Mat.Shoot0_Mat"))))

(event `self.Box.OnComponentBeginOverlap`
  (params (OverlappedComponent :type "PrimitiveComponent Object Reference") (OtherActor :type "Actor Object Reference") (OtherComp :type "PrimitiveComponent Object Reference") (OtherBodyIndex :type Integer) (bFromSweep :type Boolean) (SweepResult :type "HitResult Structure (by ref)"))
  (cast `/Game/Blueprints/SpaceEater_Pawn` OtherActor)
  (bind _asspace_eater_gstate (cast `/Game/Blueprints/SpaceEater_GState` (`GameplayStatics.GetGameState`)))
  (`/Game/Blueprints/SpaceEater_GState.RefreshDocs` _asspace_eater_gstate)
  (`/Game/Blueprints/SpaceEater_GState.Close Documents` _asspace_eater_gstate)
  (`/Game/Blueprints/SpaceEater_GState.Close UserFiles` _asspace_eater_gstate))

(fn `UserConstructionScript`)
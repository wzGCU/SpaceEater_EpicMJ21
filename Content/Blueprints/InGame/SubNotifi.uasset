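; SubNotifi is an in-game notification actor that shows a random number and is dismissed by the selection cursor.
; On BeginPlay it fills its Random text with two joined random three-digit numbers and calls Ok on the SpaceEater game instance.
; When a CursorSelect_Blueprint actor overlaps the Close component, it destroys both that cursor actor and itself.
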(event `self.ReceiveBeginPlay`
  (`TextRenderComponent.K2_SetText` (`self.Random`) (`KismetTextLibrary.Conv_StringToText` (`KismetStringLibrary.Concat_StrStr` (`KismetStringLibrary.Conv_IntToString` (`KismetMathLibrary.RandomIntegerInRange` 100 999)) (`KismetStringLibrary.Conv_IntToString` (`KismetMathLibrary.RandomIntegerInRange` 100 999)))))
  (bind _asspace_eater_ginstance (cast `/Game/Blueprints/SpaceEater_Ginstance` (`GameplayStatics.GetGameInstance`)))
  (`/Game/Blueprints/SpaceEater_Ginstance.Ok` _asspace_eater_ginstance))

(event `self.Close.OnComponentBeginOverlap`
  (params (OverlappedComponent :type "PrimitiveComponent Object Reference") (OtherActor :type "Actor Object Reference") (OtherComp :type "PrimitiveComponent Object Reference") (OtherBodyIndex :type Integer) (bFromSweep :type Boolean) (SweepResult :type "HitResult Structure (by ref)"))
  (bind _ascursor_select_blueprint (cast `/Game/Blueprints/CursorSelect_Blueprint` OtherActor))
  (`self.K2_DestroyActor` _ascursor_select_blueprint)
  (`self.K2_DestroyActor`))

(fn `UserConstructionScript`)
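; UserFiles_BP is an in-game user files actor, apparently a desktop-style window with Documents, Photos, Music and Videos entries and a Close control.
; Each is a component that reacts only to overlaps from CursorSelect_Blueprint, so selection works through collision.
; The four folder overlaps call their matching Open function on SpaceEater_GState, while Close destroys the actor.
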(event `self.Close.OnComponentBeginOverlap`
  (params (OverlappedComponent :type "PrimitiveComponent Object Reference") (OtherActor :type "Actor Object Reference") (OtherComp :type "PrimitiveComponent Object Reference") (OtherBodyIndex :type Integer) (bFromSweep :type Boolean) (SweepResult :type "HitResult Structure (by ref)"))
  (cast `/Game/Blueprints/CursorSelect_Blueprint` OtherActor)
  (`self.K2_DestroyActor`))

(event `self.Documents.OnComponentBeginOverlap`
  (params (OverlappedComponent :type "PrimitiveComponent Object Reference") (OtherActor :type "Actor Object Reference") (OtherComp :type "PrimitiveComponent Object Reference") (OtherBodyIndex :type Integer) (bFromSweep :type Boolean) (SweepResult :type "HitResult Structure (by ref)"))
  (cast `/Game/Blueprints/CursorSelect_Blueprint` OtherActor)
  (bind _asspace_eater_gstate (cast `/Game/Blueprints/SpaceEater_GState` (`GameplayStatics.GetGameState`)))
  (`/Game/Blueprints/SpaceEater_GState.OpenDocuments` _asspace_eater_gstate))

(event `self.Photos.OnComponentBeginOverlap`
  (params (OverlappedComponent :type "PrimitiveComponent Object Reference") (OtherActor :type "Actor Object Reference") (OtherComp :type "PrimitiveComponent Object Reference") (OtherBodyIndex :type Integer) (bFromSweep :type Boolean) (SweepResult :type "HitResult Structure (by ref)"))
  (cast `/Game/Blueprints/CursorSelect_Blueprint` OtherActor)
  (bind _asspace_eater_gstate (cast `/Game/Blueprints/SpaceEater_GState` (`GameplayStatics.GetGameState`)))
  (`/Game/Blueprints/SpaceEater_GState.OpenPhotos` _asspace_eater_gstate))

(event `self.Music.OnComponentBeginOverlap`
  (params (OverlappedComponent :type "PrimitiveComponent Object Reference") (OtherActor :type "Actor Object Reference") (OtherComp :type "PrimitiveComponent Object Reference") (OtherBodyIndex :type Integer) (bFromSweep :type Boolean) (SweepResult :type "HitResult Structure (by ref)"))
  (cast `/Game/Blueprints/CursorSelect_Blueprint` OtherActor)
  (bind _asspace_eater_gstate (cast `/Game/Blueprints/SpaceEater_GState` (`GameplayStatics.GetGameState`)))
  (`/Game/Blueprints/SpaceEater_GState.OpenMusic` _asspace_eater_gstate))

(event `self.Videos.OnComponentBeginOverlap`
  (params (OverlappedComponent :type "PrimitiveComponent Object Reference") (OtherActor :type "Actor Object Reference") (OtherComp :type "PrimitiveComponent Object Reference") (OtherBodyIndex :type Integer) (bFromSweep :type Boolean) (SweepResult :type "HitResult Structure (by ref)"))
  (cast `/Game/Blueprints/CursorSelect_Blueprint` OtherActor)
  (bind _asspace_eater_gstate (cast `/Game/Blueprints/SpaceEater_GState` (`GameplayStatics.GetGameState`)))
  (`/Game/Blueprints/SpaceEater_GState.OpenVideos` _asspace_eater_gstate))

(fn `UserConstructionScript`)
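; Game mode for SpaceEater that starts the HUD and ends the game when free space runs out.
; On BeginPlay it has the player controller generate the HUD.
; Each Tick it polls the game state's FreeSpace; at zero it runs a one-time game-over sequence.
; That sequence notifies the controller, stops play, closes user files, calls the pawn's JumpFolder three times, spawns GameOver_BP and stops the in-game background.
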(event `self.ReceiveBeginPlay`
  (bind _asspace_eater_pcontroller (cast `/Game/Blueprints/SpaceEater_PController` (`GameplayStatics.GetPlayerController` 0)))
  (`/Game/Blueprints/SpaceEater_PController.Generate HUD` _asspace_eater_pcontroller))

(event `self.ReceiveTick`
  (params (DeltaSeconds :type "Float (single-precision)"))
  (bind _asspace_eater_gstate (cast `/Game/Blueprints/SpaceEater_GState` (`GameplayStatics.GetGameState`)))
  (if (<= (`/Game/Blueprints/SpaceEater_GState.FreeSpace` _asspace_eater_gstate) 0.0)
    (if (not (`self.didOnceGOVER`))
      (set `self.didOnceGOVER` true)
      (bind _asspace_eater_pcontroller (cast `/Game/Blueprints/SpaceEater_PController` (`GameplayStatics.GetPlayerController` 0)))
      (`/Game/Blueprints/SpaceEater_PController.GameOver` _asspace_eater_pcontroller)
      (set `/Game/Blueprints/SpaceEater_GState.gameIsOn` false _asspace_eater_gstate)
      (`/Game/Blueprints/SpaceEater_GState.Close UserFiles` _asspace_eater_gstate)
      (bind _asspace_eater_pawn (cast `/Game/Blueprints/SpaceEater_Pawn` (`GameplayStatics.GetPlayerPawn` 0)))
      (`/Game/Blueprints/SpaceEater_Pawn.JumpFolder` _asspace_eater_pawn)
      (`/Game/Blueprints/SpaceEater_Pawn.JumpFolder` _asspace_eater_pawn)
      (`/Game/Blueprints/SpaceEater_Pawn.JumpFolder` _asspace_eater_pawn)
      (`|SpawnActorFromClass` "/Game/Blueprints/InGame/GameOver_BP.GameOver_BP_C" (`KismetMathLibrary.MakeTransform` (0.0 0.0 900.0)) "Undefined" "OverrideRootScale" null null)
      (bind _asspace_eater_ginstance (cast `/Game/Blueprints/SpaceEater_Ginstance` (`GameplayStatics.GetGameInstance`)))
      (`/Game/Blueprints/SpaceEater_Ginstance.StopInGameBG` _asspace_eater_ginstance))))

(fn `UserConstructionScript`)
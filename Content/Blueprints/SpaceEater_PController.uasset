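; SpaceEater_PController is a Blueprint, named as a player controller, that manages the HUD and game-over screen for SpaceEater.
; GenerateHUD adds a W_HUD widget to the viewport and sets game-only input, while RemoveHUD takes it down.
; GameOver swaps the HUD for a W_GOver widget, then after a fixed delay RemoveGameOver clears it and opens the Menu level.
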(event `Generate HUD`
  (bind _returnvalue (`|CreateWidget` "/Game/W_HUD.W_HUD_C"))
  (bind _output_get (set `self.HUDReference` _returnvalue))
  (`UserWidget.AddToViewport` _output_get 0)
  (`WidgetBlueprintLibrary.SetInputMode_GameOnly` self))

(event `Remove HUD`
  (`Widget.RemoveFromParent` (`self.HUDReference`)))

(event `GameOver`
  (`self.Remove HUD`)
  (bind _returnvalue (`|CreateWidget` "/Game/W_GOver.W_GOver_C"))
  (bind _output_get (set `self.GOVerReference` _returnvalue))
  (`UserWidget.AddToViewport` _output_get 0)
  (`KismetSystemLibrary.Delay` 45.0)
  (`self.Remove GameOver`))

(event `Remove GameOver`
  (`Widget.RemoveFromParent` (`self.GOVerReference`))
  (`GameplayStatics.OpenLevelBySoftObjectPtr` "/Game/Maps/Menu.Menu"))

(fn `UserConstructionScript`)
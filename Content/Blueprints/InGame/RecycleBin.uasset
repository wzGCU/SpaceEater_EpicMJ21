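; Recycle Bin window actor that shows how much space can be recovered and lets the player empty or close it.
; On begin play, it writes SpaceToRecover from SpaceEater_GState into its RecoverSpace text.
; Its Empty and Close components act as buttons triggered by CursorSelect_Blueprint overlaps.
; Empty calls RecoverSpace on the game state and refreshes the text, while Close destroys the cursor actor and calls CloseRecycleBin.
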(event `self.ReceiveBeginPlay`
  (bind _asspace_eater_gstate (cast `/Game/Blueprints/SpaceEater_GState` (`GameplayStatics.GetGameState`) :!label _label))
  (`TextRenderComponent.K2_SetText` (`self.RecoverSpace`) (`KismetTextLibrary.Conv_DoubleToText` (`/Game/Blueprints/SpaceEater_GState.SpaceToRecover` _asspace_eater_gstate) "HalfToEven" false true 1 324 1)))

(event `self.Close.OnComponentBeginOverlap`
  (params (OverlappedComponent :type "PrimitiveComponent Object Reference") (OtherActor :type "Actor Object Reference") (OtherComp :type "PrimitiveComponent Object Reference") (OtherBodyIndex :type Integer) (bFromSweep :type Boolean) (SweepResult :type "HitResult Structure (by ref)"))
  (bind _ascursor_select_blueprint (cast `/Game/Blueprints/CursorSelect_Blueprint` OtherActor))
  (`self.K2_DestroyActor` _ascursor_select_blueprint)
  (bind _asspace_eater_gstate (cast `/Game/Blueprints/SpaceEater_GState` (`GameplayStatics.GetGameState`)))
  (`/Game/Blueprints/SpaceEater_GState.CloseRecycleBin` _asspace_eater_gstate))

(event `self.Empty.OnComponentBeginOverlap`
  (params (OverlappedComponent :type "PrimitiveComponent Object Reference") (OtherActor :type "Actor Object Reference") (OtherComp :type "PrimitiveComponent Object Reference") (OtherBodyIndex :type Integer) (bFromSweep :type Boolean) (SweepResult :type "HitResult Structure (by ref)"))
  (cast `/Game/Blueprints/CursorSelect_Blueprint` OtherActor)
  (`/Game/Blueprints/SpaceEater_GState.RecoverSpace` (stale `self.ReceiveBeginPlay` _asspace_eater_gstate))
  (goto _label))

(fn `UserConstructionScript`)
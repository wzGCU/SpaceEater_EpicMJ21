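; Game state for SpaceEater, a desktop-themed game where viruses in user folders eat free disk space.
; Looping timers count run time, randomly raise capped per-category virus counts after a delay, and drain FreeSpace by their weighted sum.
; Open/Close events spawn and destroy folder windows, clean files and viruses, using chained switch cases to spawn one virus per count.
; Other events refresh virus arrays, recover space and briefly raise cat, game and readme flags.
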(event `AddVirus`
  (bind _documentsmonsters (`self.DocumentsMonsters`))
  (bind _musicmonsters (`self.MusicMonsters`))
  (bind _videosmonsters (`self.VideosMonsters`))
  (bind _photosmonsters (`self.PhotosMonsters`))
  (bind _gamemonsters (`self.GameMonsters`))
  (if (`self.gameIsOn`)
    (`KismetSystemLibrary.Delay` (`KismetMathLibrary.RandomFloatInRange` 5.0 10.0))
    (switch `int` (`KismetMathLibrary.RandomIntegerInRange` 0 4)
      (:`0`
        (if (not (>= _documentsmonsters 7))
          (`/Engine/EditorBlueprintResources/StandardMacros.IncrementInt` _documentsmonsters)))
      (:`1`
        (if (not (>= _musicmonsters 7))
          (`/Engine/EditorBlueprintResources/StandardMacros.IncrementInt` _musicmonsters)))
      (:`2`
        (if (not (>= _videosmonsters 7))
          (`/Engine/EditorBlueprintResources/StandardMacros.IncrementInt` _videosmonsters)))
      (:`3`
        (if (not (>= _photosmonsters 7))
          (`/Engine/EditorBlueprintResources/StandardMacros.IncrementInt` _photosmonsters)))
      (:`4`
        (if (not (>= _gamemonsters 3))
          (`/Engine/EditorBlueprintResources/StandardMacros.IncrementInt` _gamemonsters))))))

(event `self.ReceiveBeginPlay`
  (`KismetSystemLibrary.Delay` 2.0)
  (`KismetSystemLibrary.K2_SetTimer` null "EatSpace" 0.2 true)
  (`KismetSystemLibrary.K2_SetTimer` null "AddVirus" 3.0 true)
  (`KismetSystemLibrary.K2_SetTimer` null "SecondsRunning" 1.0 true))

(event `EatSpace`
  (if (`self.gameIsOn`)
    (set `self.FreeSpace` (- (`self.FreeSpace`) (+ (* (`self.DocumentsMonsters`) 0.05) (* (`self.VideosMonsters`) 0.2) (* (`self.PhotosMonsters`) 0.1) (* (`self.MusicMonsters`) 0.15) (* (`self.GameMonsters`) 0.4))))))

(event `Cat Action`
  (if (not (`self.cuteCatEnabled`))
    (set `self.cuteCatEnabled` true)
    (`KismetSystemLibrary.Delay` 2.0)
    (set `self.cuteCatEnabled` false)))

(event `SecondsRunning`
  (if (`self.gameIsOn`)
    (`/Engine/EditorBlueprintResources/StandardMacros.IncrementInt` (`self.TimeRunning`))))

(event `GameAction`
  (if (not (`self.gameInGame`))
    (set `self.gameInGame` true)
    (`KismetSystemLibrary.Delay` 2.0)
    (set `self.gameInGame` false)))

(event `ReadMeAction`
  (if (not (`self.README`))
    (set `self.README` true)
    (`KismetSystemLibrary.Delay` 5.0)
    (set `self.README` false)))

(event `OpenUserFiles`
  (bind _asspace_eater_pawn (cast `/Game/Blueprints/SpaceEater_Pawn` (`GameplayStatics.GetPlayerPawn` 0)))
  (`/Game/Blueprints/SpaceEater_Pawn.JumpFolder` _asspace_eater_pawn)
  (`|SpawnActorFromClass` "/Game/Blueprints/InGame/UserFiles_BP.UserFiles_BP_C" (`KismetMathLibrary.MakeTransform` (0.0 0.0 300.0)) "Undefined" "OverrideRootScale" null null))

(event `Close UserFiles`
  (bind _outactors (`GameplayStatics.GetAllActorsOfClass` "/Game/Blueprints/InGame/UserFiles_BP.UserFiles_BP_C"))
  (for _array_element _outactors
    (`self.K2_DestroyActor` _array_element)))

(event `OpenDocuments`
  ;[1 0.276 0.276] Documents
  (bind _returnvalue (`|SpawnActorFromClass` "/Game/Blueprints/InGame/Folder_Documents.Folder_Documents_C" (`KismetMathLibrary.MakeTransform` (0.0 0.0 600.0)) "Undefined" "OverrideRootScale" null null))
  (bind _asspace_eater_pawn (cast `/Game/Blueprints/SpaceEater_Pawn` (`GameplayStatics.GetPlayerPawn` 0)))
  (`/Game/Blueprints/SpaceEater_Pawn.JumpFolder` _asspace_eater_pawn)
  (`|SpawnActorFromClass` "/Game/Blueprints/Buttons/Document_Clean.Document_Clean_C" (`KismetMathLibrary.MakeTransform` (`self.File1`)) "Undefined" "OverrideRootScale" null null)
  (switch `int` (`self.DocumentsMonsters`)
    (:`1`
      _)
    (:`2`
      (bind _returnvalue_2 (`|SpawnActorFromClass` "/Game/Blueprints/Buttons/Document_VIR.Document_VIR_C" (`KismetMathLibrary.MakeTransform` (`self.File3`)) "Undefined" "OverrideRootScale" null null :!label _label))
      (`KismetArrayLibrary.Array_Add` (`self.ActiveDocumentVirus`) _returnvalue_2))
    (:`3`
      (bind _returnvalue_3 (`|SpawnActorFromClass` "/Game/Blueprints/Buttons/Document_VIR.Document_VIR_C" (`KismetMathLibrary.MakeTransform` (`self.File4`)) "Undefined" "OverrideRootScale" null null :!label _label_2))
      (`KismetArrayLibrary.Array_Add` (`self.ActiveDocumentVirus`) _returnvalue_3)
      (goto _label))
    (:`4`
      (bind _returnvalue_4 (`|SpawnActorFromClass` "/Game/Blueprints/Buttons/Document_VIR.Document_VIR_C" (`KismetMathLibrary.MakeTransform` (`self.File5`)) "Undefined" "OverrideRootScale" null null :!label _label_3))
      (`KismetArrayLibrary.Array_Add` (`self.ActiveDocumentVirus`) _returnvalue_4)
      (goto _label_2))
    (:`5`
      (bind _returnvalue_5 (`|SpawnActorFromClass` "/Game/Blueprints/Buttons/Document_VIR.Document_VIR_C" (`KismetMathLibrary.MakeTransform` (`self.File6`)) "Undefined" "OverrideRootScale" null null :!label _label_4))
      (`KismetArrayLibrary.Array_Add` (`self.ActiveDocumentVirus`) _returnvalue_5)
      (goto _label_3))
    (:`6`
      (bind _returnvalue_6 (`|SpawnActorFromClass` "/Game/Blueprints/Buttons/Document_VIR.Document_VIR_C" (`KismetMathLibrary.MakeTransform` (`self.File7`)) "Undefined" "OverrideRootScale" null null :!label _label_5))
      (`KismetArrayLibrary.Array_Add` (`self.ActiveDocumentVirus`) _returnvalue_6)
      (goto _label_4))
    (:`7`
      (bind _returnvalue_7 (`|SpawnActorFromClass` "/Game/Blueprints/Buttons/Document_VIR.Document_VIR_C" (`KismetMathLibrary.MakeTransform` (`self.File8`)) "Undefined" "OverrideRootScale" null null))
      (`KismetArrayLibrary.Array_Add` (`self.ActiveDocumentVirus`) _returnvalue_7)
      (goto _label_5)))
  (bind _returnvalue_8 (`|SpawnActorFromClass` "/Game/Blueprints/Buttons/Document_VIR.Document_VIR_C" (`KismetMathLibrary.MakeTransform` (`self.File2`)) "Undefined" "OverrideRootScale" null null))
  (`KismetArrayLibrary.Array_Add` (`self.ActiveDocumentVirus`) _returnvalue_8))

(event `Close Documents`
  ;[1 0.276 0.276] Documents
  (bind _outactors (`GameplayStatics.GetAllActorsOfClass` "/Game/Blueprints/Buttons/Document_VIR.Document_VIR_C"))
  (for _array_element _outactors
    (`self.K2_DestroyActor` _array_element))
  (bind _outactors_2 (`GameplayStatics.GetAllActorsOfClass` "/Game/Blueprints/Buttons/Document_Clean.Document_Clean_C"))
  (for _array_element_2 _outactors_2
    (`self.K2_DestroyActor` _array_element_2))
  (`KismetSystemLibrary.Delay` 0.2)
  (`self.K2_DestroyActor` (stale `OpenDocuments` _returnvalue)))

(event `RefreshDocs`
  ;[1 0.276 0.276] Documents
  (`KismetArrayLibrary.Array_Clear` (`self.ActiveDocumentVirus`))
  (bind _outactors (`GameplayStatics.GetAllActorsOfClass` "/Game/Blueprints/Buttons/Document_VIR.Document_VIR_C"))
  (set `self.ActiveDocumentVirus` _outactors))

(event `OpenVideos`
  (bind _activevideosvirus (`self.ActiveVideosVirus`))
  ;[1 0.98 0.1818] Videos
  (bind _returnvalue (`|SpawnActorFromClass` "/Game/Blueprints/InGame/Folder_Videos.Folder_Videos_C" (`KismetMathLibrary.MakeTransform` (0.0 0.0 600.0)) "Undefined" "OverrideRootScale" null null))
  (bind _asspace_eater_pawn (cast `/Game/Blueprints/SpaceEater_Pawn` (`GameplayStatics.GetPlayerPawn` 0)))
  (`/Game/Blueprints/SpaceEater_Pawn.JumpFolder` _asspace_eater_pawn)
  (bind _returnvalue_2 (`|SpawnActorFromClass` "/Game/Blueprints/Buttons/Video_Clean.Video_Clean_C" (`KismetMathLibrary.MakeTransform` (`self.File1`)) "Undefined" "OverrideRootScale" null null))
  (switch `int` (`self.VideosMonsters`)
    (:`1`
      _)
    (:`2`
      (bind _returnvalue_3 (`|SpawnActorFromClass` "/Game/Blueprints/Buttons/Video_VIR.Video_VIR_C" (`KismetMathLibrary.MakeTransform` (`self.File3`)) "Undefined" "OverrideRootScale" null null :!label _label_6))
      (`KismetArrayLibrary.Array_Add` _activevideosvirus _returnvalue_3))
    (:`3`
      (bind _returnvalue_4 (`|SpawnActorFromClass` "/Game/Blueprints/Buttons/Video_VIR.Video_VIR_C" (`KismetMathLibrary.MakeTransform` (`self.File4`)) "Undefined" "OverrideRootScale" null null :!label _label_7))
      (`KismetArrayLibrary.Array_Add` _activevideosvirus _returnvalue_4)
      (goto _label_6))
    (:`4`
      (bind _returnvalue_5 (`|SpawnActorFromClass` "/Game/Blueprints/Buttons/Video_VIR.Video_VIR_C" (`KismetMathLibrary.MakeTransform` (`self.File5`)) "Undefined" "OverrideRootScale" null null :!label _label_8))
      (`KismetArrayLibrary.Array_Add` _activevideosvirus _returnvalue_5)
      (goto _label_7))
    (:`5`
      (bind _returnvalue_6 (`|SpawnActorFromClass` "/Game/Blueprints/Buttons/Video_VIR.Video_VIR_C" (`KismetMathLibrary.MakeTransform` (`self.File6`)) "Undefined" "OverrideRootScale" null null :!label _label_9))
      (`KismetArrayLibrary.Array_Add` _activevideosvirus _returnvalue_6)
      (goto _label_8))
    (:`6`
      (bind _returnvalue_7 (`|SpawnActorFromClass` "/Game/Blueprints/Buttons/Video_VIR.Video_VIR_C" (`KismetMathLibrary.MakeTransform` (`self.File7`)) "Undefined" "OverrideRootScale" null null :!label _label_10))
      (`KismetArrayLibrary.Array_Add` _activevideosvirus _returnvalue_7)
      (goto _label_9))
    (:`7`
      (bind _returnvalue_8 (`|SpawnActorFromClass` "/Game/Blueprints/Buttons/Video_VIR.Video_VIR_C" (`KismetMathLibrary.MakeTransform` (`self.File8`)) "Undefined" "OverrideRootScale" null null))
      (`KismetArrayLibrary.Array_Add` _activevideosvirus _returnvalue_8)
      (goto _label_10)))
  (bind _returnvalue_9 (`|SpawnActorFromClass` "/Game/Blueprints/Buttons/Video_VIR.Video_VIR_C" (`KismetMathLibrary.MakeTransform` (`self.File2`)) "Undefined" "OverrideRootScale" null null))
  (`KismetArrayLibrary.Array_Add` _activevideosvirus _returnvalue_9))

(event `CloseVideos`
  ;[1 0.98 0.1818] Videos
  (for _array_element (`self.ActiveVideosVirus`)
    (`self.K2_DestroyActor` _array_element))
  (`self.K2_DestroyActor` (stale `OpenVideos` _returnvalue_2))
  (`KismetSystemLibrary.Delay` 0.2)
  (`self.K2_DestroyActor` (stale `OpenVideos` _returnvalue)))

(event `RefreshVideos`
  ;[1 0.98 0.1818] Videos
  (`KismetArrayLibrary.Array_Clear` (`self.ActiveVideosVirus`))
  (bind _outactors (`GameplayStatics.GetAllActorsOfClass` "/Game/Blueprints/Buttons/Video_VIR.Video_VIR_C"))
  (set `self.ActiveVideosVirus` _outactors))

(event `OpenPhotos`
  (bind _activephotosvirus (`self.ActivePhotosVirus`))
  ;[1 0.1062 0.9036] Photos
  (bind _returnvalue (`|SpawnActorFromClass` "/Game/Blueprints/InGame/Folder_Photos.Folder_Photos_C" (`KismetMathLibrary.MakeTransform` (0.0 0.0 600.0)) "Undefined" "OverrideRootScale" null null))
  (bind _asspace_eater_pawn (cast `/Game/Blueprints/SpaceEater_Pawn` (`GameplayStatics.GetPlayerPawn` 0)))
  (`/Game/Blueprints/SpaceEater_Pawn.JumpFolder` _asspace_eater_pawn)
  (bind _returnvalue_2 (`|SpawnActorFromClass` "/Game/Blueprints/Buttons/Photo_Clean.Photo_Clean_C" (`KismetMathLibrary.MakeTransform` (`self.File1`)) "Undefined" "OverrideRootScale" null null))
  (switch `int` (`self.PhotosMonsters`)
    (:`1`
      _)
    (:`2`
      (bind _returnvalue_3 (`|SpawnActorFromClass` "/Game/Blueprints/Buttons/Photo_VIR.Photo_VIR_C" (`KismetMathLibrary.MakeTransform` (`self.File3`)) "Undefined" "OverrideRootScale" null null :!label _label_11))
      (`KismetArrayLibrary.Array_Add` _activephotosvirus _returnvalue_3))
    (:`3`
      (bind _returnvalue_4 (`|SpawnActorFromClass` "/Game/Blueprints/Buttons/Photo_VIR.Photo_VIR_C" (`KismetMathLibrary.MakeTransform` (`self.File4`)) "Undefined" "OverrideRootScale" null null :!label _label_12))
      (`KismetArrayLibrary.Array_Add` _activephotosvirus _returnvalue_4)
      (goto _label_11))
    (:`4`
      (bind _returnvalue_5 (`|SpawnActorFromClass` "/Game/Blueprints/Buttons/Photo_VIR.Photo_VIR_C" (`KismetMathLibrary.MakeTransform` (`self.File5`)) "Undefined" "OverrideRootScale" null null :!label _label_13))
      (`KismetArrayLibrary.Array_Add` _activephotosvirus _returnvalue_5)
      (goto _label_12))
    (:`5`
      (bind _returnvalue_6 (`|SpawnActorFromClass` "/Game/Blueprints/Buttons/Photo_VIR.Photo_VIR_C" (`KismetMathLibrary.MakeTransform` (`self.File6`)) "Undefined" "OverrideRootScale" null null :!label _label_14))
      (`KismetArrayLibrary.Array_Add` _activephotosvirus _returnvalue_6)
      (goto _label_13))
    (:`6`
      (bind _returnvalue_7 (`|SpawnActorFromClass` "/Game/Blueprints/Buttons/Photo_VIR.Photo_VIR_C" (`KismetMathLibrary.MakeTransform` (`self.File7`)) "Undefined" "OverrideRootScale" null null :!label _label_15))
      (`KismetArrayLibrary.Array_Add` _activephotosvirus _returnvalue_7)
      (goto _label_14))
    (:`7`
      (bind _returnvalue_8 (`|SpawnActorFromClass` "/Game/Blueprints/Buttons/Photo_VIR.Photo_VIR_C" (`KismetMathLibrary.MakeTransform` (`self.File8`)) "Undefined" "OverrideRootScale" null null))
      (`KismetArrayLibrary.Array_Add` _activephotosvirus _returnvalue_8)
      (goto _label_15)))
  (bind _returnvalue_9 (`|SpawnActorFromClass` "/Game/Blueprints/Buttons/Photo_VIR.Photo_VIR_C" (`KismetMathLibrary.MakeTransform` (`self.File2`)) "Undefined" "OverrideRootScale" null null))
  (`KismetArrayLibrary.Array_Add` _activephotosvirus _returnvalue_9))

(event `ClosePhotos`
  ;[1 0.1062 0.9036] Photos
  (for _array_element (`self.ActivePhotosVirus`)
    (`self.K2_DestroyActor` _array_element))
  (`self.K2_DestroyActor` (stale `OpenPhotos` _returnvalue_2))
  (`KismetSystemLibrary.Delay` 0.2)
  (`self.K2_DestroyActor` (stale `OpenPhotos` _returnvalue)))

(event `RefreshPhotos`
  ;[1 0.1062 0.9036] Photos
  (`KismetArrayLibrary.Array_Clear` (`self.ActivePhotosVirus`))
  (bind _outactors (`GameplayStatics.GetAllActorsOfClass` "/Game/Blueprints/Buttons/Photo_VIR.Photo_VIR_C"))
  (set `self.ActivePhotosVirus` _outactors))

(event `OpenMusic`
  (bind _activemusicvirus (`self.ActiveMusicVirus`))
  ;[0.322 1 0.2147] Music
  (bind _returnvalue (`|SpawnActorFromClass` "/Game/Blueprints/InGame/Folder_Music.Folder_Music_C" (`KismetMathLibrary.MakeTransform` (0.0 0.0 600.0)) "Undefined" "OverrideRootScale" null null))
  (bind _asspace_eater_pawn (cast `/Game/Blueprints/SpaceEater_Pawn` (`GameplayStatics.GetPlayerPawn` 0)))
  (`/Game/Blueprints/SpaceEater_Pawn.JumpFolder` _asspace_eater_pawn)
  (bind _returnvalue_2 (`|SpawnActorFromClass` "/Game/Blueprints/Buttons/Music_Clean.Music_Clean_C" (`KismetMathLibrary.MakeTransform` (`self.File1`)) "Undefined" "OverrideRootScale" null null))
  (switch `int` (`self.MusicMonsters`)
    (:`1`
      _)
    (:`2`
      (bind _returnvalue_3 (`|SpawnActorFromClass` "/Game/Blueprints/Buttons/Music_VIR.Music_VIR_C" (`KismetMathLibrary.MakeTransform` (`self.File3`)) "Undefined" "OverrideRootScale" null null :!label _label_16))
      (`KismetArrayLibrary.Array_Add` _activemusicvirus _returnvalue_3))
    (:`3`
      (bind _returnvalue_4 (`|SpawnActorFromClass` "/Game/Blueprints/Buttons/Music_VIR.Music_VIR_C" (`KismetMathLibrary.MakeTransform` (`self.File4`)) "Undefined" "OverrideRootScale" null null :!label _label_17))
      (`KismetArrayLibrary.Array_Add` _activemusicvirus _returnvalue_4)
      (goto _label_16))
    (:`4`
      (bind _returnvalue_5 (`|SpawnActorFromClass` "/Game/Blueprints/Buttons/Music_VIR.Music_VIR_C" (`KismetMathLibrary.MakeTransform` (`self.File5`)) "Undefined" "OverrideRootScale" null null :!label _label_18))
      (`KismetArrayLibrary.Array_Add` _activemusicvirus _returnvalue_5)
      (goto _label_17))
    (:`5`
      (bind _returnvalue_6 (`|SpawnActorFromClass` "/Game/Blueprints/Buttons/Music_VIR.Music_VIR_C" (`KismetMathLibrary.MakeTransform` (`self.File6`)) "Undefined" "OverrideRootScale" null null :!label _label_19))
      (`KismetArrayLibrary.Array_Add` _activemusicvirus _returnvalue_6)
      (goto _label_18))
    (:`6`
      (bind _returnvalue_7 (`|SpawnActorFromClass` "/Game/Blueprints/Buttons/Music_VIR.Music_VIR_C" (`KismetMathLibrary.MakeTransform` (`self.File7`)) "Undefined" "OverrideRootScale" null null :!label _label_20))
      (`KismetArrayLibrary.Array_Add` _activemusicvirus _returnvalue_7)
      (goto _label_19))
    (:`7`
      (bind _returnvalue_8 (`|SpawnActorFromClass` "/Game/Blueprints/Buttons/Music_VIR.Music_VIR_C" (`KismetMathLibrary.MakeTransform` (`self.File8`)) "Undefined" "OverrideRootScale" null null))
      (`KismetArrayLibrary.Array_Add` _activemusicvirus _returnvalue_8)
      (goto _label_20)))
  (bind _returnvalue_9 (`|SpawnActorFromClass` "/Game/Blueprints/Buttons/Music_VIR.Music_VIR_C" (`KismetMathLibrary.MakeTransform` (`self.File2`)) "Undefined" "OverrideRootScale" null null))
  (`KismetArrayLibrary.Array_Add` _activemusicvirus _returnvalue_9))

(event `CloseMusic`
  ;[0.322 1 0.2147] Music
  (for _array_element (`self.ActiveMusicVirus`)
    (`self.K2_DestroyActor` _array_element))
  (`self.K2_DestroyActor` (stale `OpenMusic` _returnvalue_2))
  (`KismetSystemLibrary.Delay` 0.2)
  (`self.K2_DestroyActor` (stale `OpenMusic` _returnvalue)))

(event `RefreshMusic`
  ;[0.322 1 0.2147] Music
  (`KismetArrayLibrary.Array_Clear` (`self.ActiveMusicVirus`))
  (bind _outactors (`GameplayStatics.GetAllActorsOfClass` "/Game/Blueprints/Buttons/Music_VIR.Music_VIR_C"))
  (set `self.ActiveMusicVirus` _outactors))

(event `OpenGames`
  (bind (_file1_x _file1_y) (`KismetMathLibrary.BreakVector` (`self.File1`)))
  (bind (_file5_x _file5_y) (`KismetMathLibrary.BreakVector` (`self.File5`)))
  (bind (_file2_x _file2_y) (`KismetMathLibrary.BreakVector` (`self.File2`)))
  (bind _activegamesvirus (`self.ActiveGamesVirus`))
  (bind (_file7_x _file7_y) (`KismetMathLibrary.BreakVector` (`self.File7`)))
  ;[0.1476 0.269 1] Games
  (bind _returnvalue (`|SpawnActorFromClass` "/Game/Blueprints/InGame/Folder_Games.Folder_Games_C" (`KismetMathLibrary.MakeTransform` (0.0 0.0 300.0)) "Undefined" "OverrideRootScale" null null))
  (bind _asspace_eater_pawn (cast `/Game/Blueprints/SpaceEater_Pawn` (`GameplayStatics.GetPlayerPawn` 0)))
  (`/Game/Blueprints/SpaceEater_Pawn.JumpFolder` _asspace_eater_pawn)
  (bind _returnvalue_2 (`|SpawnActorFromClass` "/Game/Blueprints/Buttons/Game_Clean.Game_Clean_C" (`KismetMathLibrary.MakeTransform` (`KismetMathLibrary.MakeVector` _file1_x _file1_y 302.0)) "Undefined" "OverrideRootScale" null null))
  (switch `int` (`self.GameMonsters`)
    (:`1`
      _)
    (:`2`
      (bind _returnvalue_3 (`|SpawnActorFromClass` "/Game/Blueprints/Buttons/Game_VIR.Game_VIR_C" (`KismetMathLibrary.MakeTransform` (`KismetMathLibrary.MakeVector` _file5_x _file5_y 302.0)) "Undefined" "OverrideRootScale" null null :!label _label_21))
      (`KismetArrayLibrary.Array_Add` _activegamesvirus _returnvalue_3))
    (:`3`
      (bind _returnvalue_4 (`|SpawnActorFromClass` "/Game/Blueprints/Buttons/Game_VIR.Game_VIR_C" (`KismetMathLibrary.MakeTransform` (`KismetMathLibrary.MakeVector` _file7_x _file7_y 302.0)) "Undefined" "OverrideRootScale" null null))
      (`KismetArrayLibrary.Array_Add` _activegamesvirus _returnvalue_4)
      (goto _label_21)))
  (bind _returnvalue_5 (`|SpawnActorFromClass` "/Game/Blueprints/Buttons/Game_VIR.Game_VIR_C" (`KismetMathLibrary.MakeTransform` (`KismetMathLibrary.MakeVector` _file2_x _file2_y 302.0)) "Undefined" "OverrideRootScale" null null))
  (`KismetArrayLibrary.Array_Add` _activegamesvirus _returnvalue_5))

(event `CloseGames`
  ;[0.1476 0.269 1] Games
  (for _array_element (`self.ActiveGamesVirus`)
    (`self.K2_DestroyActor` _array_element))
  (`self.K2_DestroyActor` (stale `OpenGames` _returnvalue_2))
  (`KismetSystemLibrary.Delay` 0.2)
  (`self.K2_DestroyActor` (stale `OpenGames` _returnvalue)))

(event `RefreshGames`
  ;[0.1476 0.269 1] Games
  (`KismetArrayLibrary.Array_Clear` (`self.ActiveGamesVirus`))
  (bind _outactors (`GameplayStatics.GetAllActorsOfClass` "/Game/Blueprints/Buttons/Game_VIR.Game_VIR_C"))
  (set `self.ActiveGamesVirus` _outactors))

(event `OpenRecycleBin`
  (bind _returnvalue (`|SpawnActorFromClass` "/Game/Blueprints/InGame/RecycleBin.RecycleBin_C" (`KismetMathLibrary.MakeTransform` (0.0 0.0 300.0)) "Undefined" "OverrideRootScale" null null))
  (bind _asspace_eater_pawn (cast `/Game/Blueprints/SpaceEater_Pawn` (`GameplayStatics.GetPlayerPawn` 0)))
  (`/Game/Blueprints/SpaceEater_Pawn.JumpFolder` _asspace_eater_pawn))

(event `CloseRecycleBin`
  (`self.K2_DestroyActor` (stale `OpenRecycleBin` _returnvalue)))

(event `RecoverSpace`
  (set `self.FreeSpace` (+ (`self.SpaceToRecover`) (`self.FreeSpace`)))
  (set `self.SpaceToRecover` 0.0))

(event `OpenSub`
  (`|SpawnActorFromClass` "/Game/Blueprints/InGame/SubNotifi.SubNotifi_C" (`KismetMathLibrary.MakeTransform` (0.0 0.0 900.0)) "Undefined" "OverrideRootScale" null null)
  (bind _asspace_eater_pawn (cast `/Game/Blueprints/SpaceEater_Pawn` (`GameplayStatics.GetPlayerPawn` 0)))
  (`/Game/Blueprints/SpaceEater_Pawn.JumpFolder` _asspace_eater_pawn))

(fn `UserConstructionScript`)
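; Game_VIR is a destructible game-monster actor in SpaceEater that takes hits from CursorSelect actors.
; Each box overlap with one destroys that actor, lowers HP, and swaps the TextRender to a joke software error or status message for the remaining HP.
; At zero HP it destroys itself, decrements the GameState's monster count, calls RefreshGames, and adds points and recoverable space.
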(event `self.Box.OnComponentBeginOverlap`
  (params (OverlappedComponent :type "PrimitiveComponent Object Reference") (OtherActor :type "Actor Object Reference") (OtherComp :type "PrimitiveComponent Object Reference") (OtherBodyIndex :type Integer) (bFromSweep :type Boolean) (SweepResult :type "HitResult Structure (by ref)"))
  (bind _textrender (`self.TextRender`))
  (bind _ascursor_select_blueprint (cast `/Game/Blueprints/CursorSelect_Blueprint` OtherActor))
  (`self.K2_DestroyActor` _ascursor_select_blueprint)
  (`/Engine/EditorBlueprintResources/StandardMacros.DecrementInt` (`self.HP`)
    (:`  `
      (switch `int` (`self.HP`)
        (:`0`
          (bind _asspace_eater_gstate (cast `/Game/Blueprints/SpaceEater_GState` (`GameplayStatics.GetGameState`)))
          (`/Engine/EditorBlueprintResources/StandardMacros.DecrementInt` (`/Game/Blueprints/SpaceEater_GState.GameMonsters` _asspace_eater_gstate)
            (:`  `
              (`self.K2_DestroyActor`)
              (`/Game/Blueprints/SpaceEater_GState.RefreshGames` _asspace_eater_gstate)
              (set `/Game/Blueprints/SpaceEater_GState.Points` (+ (`/Game/Blueprints/SpaceEater_GState.Points` _asspace_eater_gstate) 5) _asspace_eater_gstate)
              (set `/Game/Blueprints/SpaceEater_GState.SpaceToRecover` (+ (`/Game/Blueprints/SpaceEater_GState.SpaceToRecover` _asspace_eater_gstate) 5.0) _asspace_eater_gstate))))
        (:`1`
          (`TextRenderComponent.K2_SetText` _textrender "### CRASH ###"))
        (:`2`
          (`TextRenderComponent.K2_SetText` _textrender "Do you want to save these files?"))
        (:`3`
          (`TextRenderComponent.K2_SetText` _textrender " LIGHTING NEEDS TO BE REBUILD"))
        (:`4`
          (`TextRenderComponent.K2_SetText` _textrender " Reading C++ Symbols"))))))

(fn `UserConstructionScript`)
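; Settings screen actor whose overlap zones let a CursorSelect_Blueprint choose sound and music volume, with an Accept zone that opens the Menu level.
; Each zone writes a preset level to SpaceEater_Ginstance's SoundsMusicVol or BgMusicVol.
; Sound zones then call Ok, presumably as an audible sample.
; Music zones restart MenuBG as a preview and stop it after a two-second delay.
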(event `self.Accept.OnComponentBeginOverlap`
  (params (OverlappedComponent :type "PrimitiveComponent Object Reference") (OtherActor :type "Actor Object Reference") (OtherComp :type "PrimitiveComponent Object Reference") (OtherBodyIndex :type Integer) (bFromSweep :type Boolean) (SweepResult :type "HitResult Structure (by ref)"))
  (cast `/Game/Blueprints/CursorSelect_Blueprint` OtherActor)
  (`GameplayStatics.OpenLevelBySoftObjectPtr` "/Game/Maps/Menu.Menu"))

(event `self.Sound20.OnComponentBeginOverlap`
  (params (OverlappedComponent :type "PrimitiveComponent Object Reference") (OtherActor :type "Actor Object Reference") (OtherComp :type "PrimitiveComponent Object Reference") (OtherBodyIndex :type Integer) (bFromSweep :type Boolean) (SweepResult :type "HitResult Structure (by ref)"))
  (cast `/Game/Blueprints/CursorSelect_Blueprint` OtherActor)
  (bind _asspace_eater_ginstance (cast `/Game/Blueprints/SpaceEater_Ginstance` (`GameplayStatics.GetGameInstance`)))
  (set `/Game/Blueprints/SpaceEater_Ginstance.soundsMusicVol` 0.2 _asspace_eater_ginstance)
  (`/Game/Blueprints/SpaceEater_Ginstance.Ok` _asspace_eater_ginstance)
  (`KismetSystemLibrary.Delay` 1.0))

(event `self.Sound40.OnComponentBeginOverlap`
  (params (OverlappedComponent :type "PrimitiveComponent Object Reference") (OtherActor :type "Actor Object Reference") (OtherComp :type "PrimitiveComponent Object Reference") (OtherBodyIndex :type Integer) (bFromSweep :type Boolean) (SweepResult :type "HitResult Structure (by ref)"))
  (cast `/Game/Blueprints/CursorSelect_Blueprint` OtherActor)
  (bind _asspace_eater_ginstance (cast `/Game/Blueprints/SpaceEater_Ginstance` (`GameplayStatics.GetGameInstance`)))
  (set `/Game/Blueprints/SpaceEater_Ginstance.soundsMusicVol` 0.4 _asspace_eater_ginstance)
  (`/Game/Blueprints/SpaceEater_Ginstance.Ok` _asspace_eater_ginstance)
  (`KismetSystemLibrary.Delay` 1.0))

(event `self.Sound60.OnComponentBeginOverlap`
  (params (OverlappedComponent :type "PrimitiveComponent Object Reference") (OtherActor :type "Actor Object Reference") (OtherComp :type "PrimitiveComponent Object Reference") (OtherBodyIndex :type Integer) (bFromSweep :type Boolean) (SweepResult :type "HitResult Structure (by ref)"))
  (cast `/Game/Blueprints/CursorSelect_Blueprint` OtherActor)
  (bind _asspace_eater_ginstance (cast `/Game/Blueprints/SpaceEater_Ginstance` (`GameplayStatics.GetGameInstance`)))
  (set `/Game/Blueprints/SpaceEater_Ginstance.soundsMusicVol` 0.6 _asspace_eater_ginstance)
  (`/Game/Blueprints/SpaceEater_Ginstance.Ok` _asspace_eater_ginstance)
  (`KismetSystemLibrary.Delay` 1.0))

(event `self.Sound80.OnComponentBeginOverlap`
  (params (OverlappedComponent :type "PrimitiveComponent Object Reference") (OtherActor :type "Actor Object Reference") (OtherComp :type "PrimitiveComponent Object Reference") (OtherBodyIndex :type Integer) (bFromSweep :type Boolean) (SweepResult :type "HitResult Structure (by ref)"))
  (cast `/Game/Blueprints/CursorSelect_Blueprint` OtherActor)
  (bind _asspace_eater_ginstance (cast `/Game/Blueprints/SpaceEater_Ginstance` (`GameplayStatics.GetGameInstance`)))
  (set `/Game/Blueprints/SpaceEater_Ginstance.soundsMusicVol` 0.8 _asspace_eater_ginstance)
  (`/Game/Blueprints/SpaceEater_Ginstance.Ok` _asspace_eater_ginstance)
  (`KismetSystemLibrary.Delay` 1.0))

(event `self.Sound100.OnComponentBeginOverlap`
  (params (OverlappedComponent :type "PrimitiveComponent Object Reference") (OtherActor :type "Actor Object Reference") (OtherComp :type "PrimitiveComponent Object Reference") (OtherBodyIndex :type Integer) (bFromSweep :type Boolean) (SweepResult :type "HitResult Structure (by ref)"))
  (cast `/Game/Blueprints/CursorSelect_Blueprint` OtherActor)
  (bind _asspace_eater_ginstance (cast `/Game/Blueprints/SpaceEater_Ginstance` (`GameplayStatics.GetGameInstance`)))
  (set `/Game/Blueprints/SpaceEater_Ginstance.soundsMusicVol` 1.0 _asspace_eater_ginstance)
  (`/Game/Blueprints/SpaceEater_Ginstance.Ok` _asspace_eater_ginstance)
  (`KismetSystemLibrary.Delay` 1.0))

(event `self.Music20.OnComponentBeginOverlap`
  (params (OverlappedComponent :type "PrimitiveComponent Object Reference") (OtherActor :type "Actor Object Reference") (OtherComp :type "PrimitiveComponent Object Reference") (OtherBodyIndex :type Integer) (bFromSweep :type Boolean) (SweepResult :type "HitResult Structure (by ref)"))
  (cast `/Game/Blueprints/CursorSelect_Blueprint` OtherActor)
  (bind _asspace_eater_ginstance (cast `/Game/Blueprints/SpaceEater_Ginstance` (`GameplayStatics.GetGameInstance`)))
  (set `/Game/Blueprints/SpaceEater_Ginstance.bgMusicVol` 0.2 _asspace_eater_ginstance)
  (`/Game/Blueprints/SpaceEater_Ginstance.StopMenuBG` _asspace_eater_ginstance)
  (`/Game/Blueprints/SpaceEater_Ginstance.MenuBG` _asspace_eater_ginstance)
  (`KismetSystemLibrary.Delay` 2.0)
  (`/Game/Blueprints/SpaceEater_Ginstance.StopMenuBG` _asspace_eater_ginstance))

(event `self.Music40.OnComponentBeginOverlap`
  (params (OverlappedComponent :type "PrimitiveComponent Object Reference") (OtherActor :type "Actor Object Reference") (OtherComp :type "PrimitiveComponent Object Reference") (OtherBodyIndex :type Integer) (bFromSweep :type Boolean) (SweepResult :type "HitResult Structure (by ref)"))
  (cast `/Game/Blueprints/CursorSelect_Blueprint` OtherActor)
  (bind _asspace_eater_ginstance (cast `/Game/Blueprints/SpaceEater_Ginstance` (`GameplayStatics.GetGameInstance`)))
  (set `/Game/Blueprints/SpaceEater_Ginstance.bgMusicVol` 0.4 _asspace_eater_ginstance)
  (`/Game/Blueprints/SpaceEater_Ginstance.StopMenuBG` _asspace_eater_ginstance)
  (`/Game/Blueprints/SpaceEater_Ginstance.MenuBG` _asspace_eater_ginstance)
  (`KismetSystemLibrary.Delay` 2.0)
  (`/Game/Blueprints/SpaceEater_Ginstance.StopMenuBG` _asspace_eater_ginstance))

(event `self.Music60.OnComponentBeginOverlap`
  (params (OverlappedComponent :type "PrimitiveComponent Object Reference") (OtherActor :type "Actor Object Reference") (OtherComp :type "PrimitiveComponent Object Reference") (OtherBodyIndex :type Integer) (bFromSweep :type Boolean) (SweepResult :type "HitResult Structure (by ref)"))
  (cast `/Game/Blueprints/CursorSelect_Blueprint` OtherActor)
  (bind _asspace_eater_ginstance (cast `/Game/Blueprints/SpaceEater_Ginstance` (`GameplayStatics.GetGameInstance`)))
  (set `/Game/Blueprints/SpaceEater_Ginstance.bgMusicVol` 0.6 _asspace_eater_ginstance)
  (`/Game/Blueprints/SpaceEater_Ginstance.StopMenuBG` _asspace_eater_ginstance)
  (`/Game/Blueprints/SpaceEater_Ginstance.MenuBG` _asspace_eater_ginstance)
  (`KismetSystemLibrary.Delay` 2.0)
  (`/Game/Blueprints/SpaceEater_Ginstance.StopMenuBG` _asspace_eater_ginstance))

(event `self.Music80.OnComponentBeginOverlap`
  (params (OverlappedComponent :type "PrimitiveComponent Object Reference") (OtherActor :type "Actor Object Reference") (OtherComp :type "PrimitiveComponent Object Reference") (OtherBodyIndex :type Integer) (bFromSweep :type Boolean) (SweepResult :type "HitResult Structure (by ref)"))
  (cast `/Game/Blueprints/CursorSelect_Blueprint` OtherActor)
  (bind _asspace_eater_ginstance (cast `/Game/Blueprints/SpaceEater_Ginstance` (`GameplayStatics.GetGameInstance`)))
  (set `/Game/Blueprints/SpaceEater_Ginstance.bgMusicVol` 0.8 _asspace_eater_ginstance)
  (`/Game/Blueprints/SpaceEater_Ginstance.StopMenuBG` _asspace_eater_ginstance)
  (`/Game/Blueprints/SpaceEater_Ginstance.MenuBG` _asspace_eater_ginstance)
  (`KismetSystemLibrary.Delay` 2.0)
  (`/Game/Blueprints/SpaceEater_Ginstance.StopMenuBG` _asspace_eater_ginstance))

(event `self.Music100.OnComponentBeginOverlap`
  (params (OverlappedComponent :type "PrimitiveComponent Object Reference") (OtherActor :type "Actor Object Reference") (OtherComp :type "PrimitiveComponent Object Reference") (OtherBodyIndex :type Integer) (bFromSweep :type Boolean) (SweepResult :type "HitResult Structure (by ref)"))
  (cast `/Game/Blueprints/CursorSelect_Blueprint` OtherActor)
  (bind _asspace_eater_ginstance (cast `/Game/Blueprints/SpaceEater_Ginstance` (`GameplayStatics.GetGameInstance`)))
  (set `/Game/Blueprints/SpaceEater_Ginstance.bgMusicVol` 1.0 _asspace_eater_ginstance)
  (`/Game/Blueprints/SpaceEater_Ginstance.StopMenuBG` _asspace_eater_ginstance)
  (`/Game/Blueprints/SpaceEater_Ginstance.MenuBG` _asspace_eater_ginstance)
  (`KismetSystemLibrary.Delay` 2.0)
  (`/Game/Blueprints/SpaceEater_Ginstance.StopMenuBG` _asspace_eater_ginstance))

(fn `UserConstructionScript`)
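; TextRenderActor_Blueprint is a world text actor that displays the current time as hours and minutes.
; BeginPlay starts a loop that rewrites the TextRender with the system time every five seconds.
; When a CursorSelect_Blueprint overlaps its Box, it shows a surprise "Boo!" message and destroys that actor.
; After a short delay the overlap path re-enters the clock loop.
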(event `self.ReceiveBeginPlay`
  (bind (_year _month _day _hour _minute) (`KismetMathLibrary.BreakDateTime` (`KismetMathLibrary.Now`)))
  (`TextRenderComponent.K2_SetText` (`self.TextRender`) (`KismetTextLibrary.Conv_StringToText` (`KismetStringLibrary.Concat_StrStr` (`KismetStringLibrary.Concat_StrStr` (`KismetTextLibrary.Conv_TextToString` (`KismetTextLibrary.Conv_IntToText` _hour false true 2)) " : ") (`KismetTextLibrary.Conv_TextToString` (`KismetTextLibrary.Conv_IntToText` _minute false true 2)))) :!label _label)
  (`KismetSystemLibrary.Delay` 5.0)
  (goto _label))

(event `self.Box.OnComponentBeginOverlap`
  (params (OverlappedComponent :type "PrimitiveComponent Object Reference") (OtherActor :type "Actor Object Reference") (OtherComp :type "PrimitiveComponent Object Reference") (OtherBodyIndex :type Integer) (bFromSweep :type Boolean) (SweepResult :type "HitResult Structure (by ref)"))
  (bind _ascursor_select_blueprint (cast `/Game/Blueprints/CursorSelect_Blueprint` OtherActor))
  (`TextRenderComponent.K2_SetText` (`self.TextRender`) (`KismetTextLibrary.Conv_StringToText` "Boo! :O"))
  (`self.K2_DestroyActor` _ascursor_select_blueprint)
  (`KismetSystemLibrary.Delay` 3.0)
  (goto _label))

(fn `UserConstructionScript`)
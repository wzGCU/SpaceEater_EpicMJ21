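; SpaceEater game instance that provides shared audio events and an intro skip for the Space Eater game.
; Separate events start and stop the gameplay and menu music from stored 2D audio components, using separate volume variables for music and effects.
; NeverGonna plays the SPAMM sound, then starts gameplay music after a short delay, while Ok plays a one-shot sound.
; IntroSkipper calls JumpFolder on the player pawn and spawns SkipIntro_BP.
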(event `InGameBGSong`
  (bind _returnvalue (`GameplayStatics.CreateSound2D` "/Game/Audios/SpaceEater.SpaceEater" (`self.bgMusicVol`) 1.0 0.0 null false false))
  (`AudioComponent.Play` _returnvalue 0.0))

(event `StopInGameBG`
  (`AudioComponent.Stop` (stale `InGameBGSong` _returnvalue)))

(event `NeverGonna`
  (bind _returnvalue (`GameplayStatics.CreateSound2D` "/Game/Audios/SPAMM.SPAMM" (`self.soundsMusicVol`) 1.0 0.0 null))
  (`AudioComponent.Play` _returnvalue 0.0)
  (`KismetSystemLibrary.Delay` 3.0)
  (`self.InGameBGSong`))

(event `Ok`
  (bind _returnvalue (`GameplayStatics.CreateSound2D` "/Game/Audios/Ok.Ok" (`self.soundsMusicVol`) 1.0 0.0 null))
  (`AudioComponent.Play` _returnvalue 0.0))

(event `MenuBG`
  (bind _returnvalue (`GameplayStatics.CreateSound2D` "/Game/Audios/SpaceEaterBGMenu.SpaceEaterBGMenu" (`self.bgMusicVol`) 1.0 0.0 null false false))
  (`AudioComponent.Play` _returnvalue 0.0))

(event `StopMenuBG`
  (`AudioComponent.Stop` (stale `MenuBG` _returnvalue)))

(event `IntroSkipper`
  (bind _asspace_eater_pawn (cast `/Game/Blueprints/SpaceEater_Pawn` (`GameplayStatics.GetPlayerPawn` 0)))
  (`/Game/Blueprints/SpaceEater_Pawn.JumpFolder` _asspace_eater_pawn)
  (`|SpawnActorFromClass` "/Game/Blueprints/InGame/SkipIntro_BP.SkipIntro_BP_C" (`KismetMathLibrary.MakeTransform` (0.0 0.0 300.0)) "Undefined" "OverrideRootScale" null null))
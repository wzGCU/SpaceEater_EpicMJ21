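; SoundsCross is a HUD marker Blueprint that shows the current SoundsMusicVol setting through the position of its static mesh.
; Every Tick it reads that value from the SpaceEater_Ginstance game instance, multiplies it by ten and rounds up.
; Even steps from 2 to 10 teleport the mesh to hardcoded world positions along the X axis; other values leave it in place.
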(event `self.ReceiveTick`
  (params (DeltaSeconds :type "Float (single-precision)"))
  (bind _staticmeshcomponent (`self.StaticMeshComponent`))
  (bind _asspace_eater_ginstance (cast `/Game/Blueprints/SpaceEater_Ginstance` (`GameplayStatics.GetGameInstance`)))
  (switch `int` (`KismetMathLibrary.Conv_Int64ToInt` (`KismetMathLibrary.FCeil64` (* (`/Game/Blueprints/SpaceEater_Ginstance.soundsMusicVol` _asspace_eater_ginstance) 10.0)))
    (:`2`
      (`SceneComponent.K2_SetWorldLocation` _staticmeshcomponent (-1235.0 110.0 107.0) false true))
    (:`4`
      (`SceneComponent.K2_SetWorldLocation` _staticmeshcomponent (-1025.0 110.0 107.0) false true))
    (:`6`
      (`SceneComponent.K2_SetWorldLocation` _staticmeshcomponent (-810.0 110.0 107.0) false true))
    (:`8`
      (`SceneComponent.K2_SetWorldLocation` _staticmeshcomponent (-595.0 110.0 107.0) false true))
    (:`10`
      (`SceneComponent.K2_SetWorldLocation` _staticmeshcomponent (-380.0 110.0 107.0) false true))))

(fn `UserConstructionScript`)
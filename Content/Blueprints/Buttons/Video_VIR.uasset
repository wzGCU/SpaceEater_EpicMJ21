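; Video_VIR is a clickable-style actor, apparently a virus video item in Space Eater, that is removed when a cursor selection actor touches it.
; Its Box overlap destroys the CursorSelect_Blueprint actor, decrements the VideosMonsters count on SpaceEater_GState and destroys itself.
; It then refreshes the videos through the game state, awards points, increases SpaceToRecover and calls OpenSub.
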(event `self.Box.OnComponentBeginOverlap`
  (params (OverlappedComponent :type "PrimitiveComponent Object Reference") (OtherActor :type "Actor Object Reference") (OtherComp :type "PrimitiveComponent Object Reference") (OtherBodyIndex :type Integer) (bFromSweep :type Boolean) (SweepResult :type "HitResult Structure (by ref)"))
  (bind _ascursor_select_blueprint (cast `/Game/Blueprints/CursorSelect_Blueprint` OtherActor))
  (`self.K2_DestroyActor` _ascursor_select_blueprint)
  (bind _asspace_eater_gstate (cast `/Game/Blueprints/SpaceEater_GState` (`GameplayStatics.GetGameState`)))
  (`/Engine/EditorBlueprintResources/StandardMacros.DecrementInt` (`/Game/Blueprints/SpaceEater_GState.VideosMonsters` _asspace_eater_gstate)
    (:`  `
      (`self.K2_DestroyActor`)
      (`/Game/Blueprints/SpaceEater_GState.RefreshVideos` _asspace_eater_gstate)
      (set `/Game/Blueprints/SpaceEater_GState.Points` (+ (`/Game/Blueprints/SpaceEater_GState.Points` _asspace_eater_gstate) 5) _asspace_eater_gstate)
      (set `/Game/Blueprints/SpaceEater_GState.SpaceToRecover` (+ (`/Game/Blueprints/SpaceEater_GState.SpaceToRecover` _asspace_eater_gstate) 1.0) _asspace_eater_gstate)
      (`/Game/Blueprints/SpaceEater_GState.OpenSub` _asspace_eater_gstate))))

(fn `UserConstructionScript`)